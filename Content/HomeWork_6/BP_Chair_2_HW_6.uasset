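; BP_Chair_2_HW_6 is a chair actor that rocks back and forth and reports its product details.
; StartSwinging prints the brand, size and price from ChairParams, then plays the Swing timeline, which drives the Chair component's relative pitch.
; StopSwinging halts the timeline.
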(event EventStartSwinging
  (Utilities|ShowChairParams)
  (bind _swing (Timeline|Swing Play)
    (:Update
      (Transformation|SetRelativeRotation (Variables|Default|GetChair) (Math|Rotator|MakeRotator 0.0 _swing 0.0) false false))))

(event EventStopSwinging
  (bind _swing (Timeline|Swing Stop)
    (:Update
      (Transformation|SetRelativeRotation (Variables|Default|GetChair) (Math|Rotator|MakeRotator 0.0 _swing 0.0) false false))))

(fn ConstructionScript)