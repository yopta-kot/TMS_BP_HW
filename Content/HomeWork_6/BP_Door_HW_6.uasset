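; BP_Door_HW_6 is a puzzle door that the player unlocks by guessing a randomly chosen key, then opens and closes.
; A box overlap toggles input, letting keys 1–3 submit guesses that are blocked during feedback or once the key is found.
; A timeline flashes the point light green or red for each guess.
; After a match, E alternately plays and reverses a timeline that rotates the door's yaw.
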(event OnComponentBeginOverlap(Box)
  (params (OverlappedComponent :type Primitive%20Component%20Object%20Reference) (OtherActor :type Actor%20Object%20Reference) (OtherComp :type Primitive%20Component%20Object%20Reference) (OtherBodyIndex :type Integer) (bFromSweep :type Boolean) (SweepResult :type Hit%20Result%20Structure%20%28by%20ref%29))
  ;[1 1 1] Enable player input
  (Input|EnableInput (Game|GetPlayerController 0)))

(event OnComponentEndOverlap(Box)
  (params (OverlappedComponent :type Primitive%20Component%20Object%20Reference) (OtherActor :type Actor%20Object%20Reference) (OtherComp :type Primitive%20Component%20Object%20Reference) (OtherBodyIndex :type Integer))
  ;[1 1 1] Disable player input
  (Input|DisableInput (Game|GetPlayerController 0)))

(event Custom|ChangePlayerKey
  (bind _pointlight (Variables|Default|GetPointLight))
  ;[1 1 1] Check player door key and current door key
  (bind _output_get (Variables|Door|SetKeysEqual? (Utilities|Enum|Equal(Enum) (Variables|Door|GetPlayerDoorKey) (Variables|Door|GetCurrentDoorKey))))
  (if _output_get
    ;[1 1 1] Setting light color depending on choicen player key
    (Rendering|Components|Light|SetLightColor _pointlight "(R=0.099045,G=1.000000,B=0.000000,A=1.000000)" true)
    (else
      (Rendering|Components|Light|SetLightColor _pointlight "(R=1.000000,G=0.000000,B=0.012242,A=1.000000)" true)))
  ;[1 1 1] Set IsFlashing as True and start animation
  (Variables|Door|SetIsFlashing? true)
  (bind _intensitymultiplier (Timeline|Flashing PlayFromStart)
    (:Update
      ;[1 1 1] Change light intesity
      (Rendering|Components|Light|SetIntensity _pointlight (* 5e+03 _intensitymultiplier)))
    (:Finished
      ;[1 1 1] Set IsFlashing as False by animation finished
      (Variables|Door|SetIsFlashing? false)
      (if (Variables|Door|GetKeysEqual?)
        ;[1 1 1] Set IsKeyFound as True if keys are equal
        (Variables|Door|SetIsKeyFound? true)
        (else
          ;[1 1 1] Set default light color if keys are not equal
          (Rendering|Components|Light|SetLightColor _pointlight "(R=1.000000,G=1.000000,B=1.000000,A=1.000000)" true))))))

(event EventBeginPlay
  ;[1 1 1] Set random door key
  (Variables|Door|SetCurrentDoorKey (Utilities|Enum|ByteToEnumEDoorKey_HW_6 (Math|Conversions|ToByte(Integer) (Math|Random|RandomIntegerinRange 0 2)))))

(event Input|KeyboardEvents|1
  (params (Key :type Key%20Structure :default "None"))
  ;[1 1 1] Set player door key
  (:Pressed
    (Variables|Door|SetPlayerDoorKey "NewEnumerator0")
    ;[1 1 1] Check to change player key
    (if (and (not (Variables|Door|GetIsKeyFound?)) (not (Variables|Door|GetIsFlashing?)))
      (CallFunction|ChangePlayerKey))))

(event Input|KeyboardEvents|2
  (params (Key :type Key%20Structure :default "None"))
  ;[1 1 1] Set player door key
  (:Pressed
    (Variables|Door|SetPlayerDoorKey "NewEnumerator1")
    ;[1 1 1] Check to change player key
    (if (and (not (Variables|Door|GetIsKeyFound?)) (not (Variables|Door|GetIsFlashing?)))
      (CallFunction|ChangePlayerKey))))

(event Input|KeyboardEvents|3
  (params (Key :type Key%20Structure :default "None"))
  ;[1 1 1] Set player door key
  (:Pressed
    (Variables|Door|SetPlayerDoorKey "NewEnumerator2")
    ;[1 1 1] Check to change player key
    (if (and (not (Variables|Door|GetIsKeyFound?)) (not (Variables|Door|GetIsFlashing?)))
      (CallFunction|ChangePlayerKey))))

(event Input|KeyboardEvents|E
  (params (Key :type Key%20Structure :default "None"))
  (:Pressed
    ;[1 1 1] If key found
    (if (Variables|Door|GetIsKeyFound?)
      ;[1 1 1] Then open or close door
      (Utilities|FlowControl|FlipFlop
        (:A
          (bind _angle (Timeline|OpenCloseDoor Play)
            (:Update
              (Transformation|SetRelativeRotation (Variables|Default|GetDoor) (Math|Rotator|MakeRotator 0.0 0.0 _angle) false false))))
        (:B
          (Timeline|OpenCloseDoor Reverse))))))

(fn ConstructionScript)